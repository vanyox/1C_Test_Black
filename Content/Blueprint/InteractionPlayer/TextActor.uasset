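; TextActor is an actor that displays configurable text through a widget component.
; Its SetText function casts the component's widget to TextW and passes the actor's text, color and font size variables to it.
; SetText runs in the construction script and again on BeginPlay, so the text is applied both when the actor is constructed and at game start.
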(event `self.ReceiveBeginPlay`
  (`self.Set Text`))

(fn `Set Text`
  (bind _astext_w (cast `/Game/Blueprint/Ui/TextW` (`WidgetComponent.GetWidget` (`self.Widget`))))
  (`/Game/Blueprint/Ui/TextW.Set Text` _astext_w (`self.Text`) (`self.Specified Color`) (`self.Font`)))

(fn `UserConstructionScript`
  (`self.Set Text`))