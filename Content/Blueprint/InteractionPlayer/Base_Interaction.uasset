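; Base interactable actor that registers itself with the GG character while that character is inside its TraceCollision volume.
; On begin overlap it stores the character, adds itself to InteractMass and switches on the character's TimerTrace.
; On end overlap it clears the reference and removes itself, switching TimerTrace off once the array is empty.
; Interact is an empty event, InteractionActor only prints debug text, and a function sets the Active flag.
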(event `InteractionActor`
  (`KismetSystemLibrary.PrintString` "INTEract" true true (struct :`B` 1.0 :`A` 1.0) 123.0))

(event `self.Trace Collision.OnComponentBeginOverlap`
  (params (OverlappedComponent :type "PrimitiveComponent Object Reference") (OtherActor :type "Actor Object Reference") (OtherComp :type "PrimitiveComponent Object Reference") (OtherBodyIndex :type Integer) (bFromSweep :type Boolean) (SweepResult :type "HitResult Structure (by ref)"))
  (bind _asgg (cast `/Game/Blueprint/Character/GG` OtherActor))
  (`/Game/Blueprint/Libraries/Interface/Char_Info.Target interact ` _asgg)
  (`KismetArrayLibrary.Array_Add` (`/Game/Blueprint/Character/GG.interact mass` _asgg) self)
  (`/Game/Blueprint/Character/GG.Timer Trace` _asgg true))

(event `self.Trace Collision.OnComponentEndOverlap`
  (params (OverlappedComponent :type "PrimitiveComponent Object Reference") (OtherActor :type "Actor Object Reference") (OtherComp :type "PrimitiveComponent Object Reference") (OtherBodyIndex :type Integer))
  (bind _asgg (cast `/Game/Blueprint/Character/GG` OtherActor))
  (`/Game/Blueprint/Libraries/Interface/Char_Info.Target interact ` null)
  (bind _interact_mass (`/Game/Blueprint/Character/GG.interact mass` _asgg))
  (if (`KismetArrayLibrary.Array_Contains` _interact_mass self)
    (`KismetArrayLibrary.Array_RemoveItem` _interact_mass self)
    (if (== (`KismetArrayLibrary.Array_Length` _interact_mass) 0)
      (`/Game/Blueprint/Character/GG.Timer Trace` _asgg false))))

(event `/Game/Blueprint/Libraries/Interface/Char_Info.Target interact `
  (params (Traget :type "/Game/Blueprint/Character/GG Object Reference"))
  (set `self.Character` Traget))

(event `/Game/Blueprint/Libraries/Interface/Char_Info.Interact`
  (params (Interact :type "/Game/Blueprint/Data/Enum/ETypeInteract Enum" :default "NewEnumerator0")))

(fn `Active/Deactive Interaction`
  (params (`Active?` :type Boolean))
  (set `self.Active?` `Active?`))

(fn `UserConstructionScript`)