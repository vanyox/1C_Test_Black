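; Interactable button in a numbered chain, where each press plays a Level Sequence and can unlock the next button.
; Interacting works once, animating the sphere by timeline, then starting the sequence, disabling itself and, after an optional delay, activating the button with the following index.
; Construction invalidates duplicate indices and reads sequence and delay from a data table row.
; A text widget shows the button number in green or red by active state.
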(event `self.ReceiveBeginPlay`
  (`self.Set info Widget`))

(event `Active Sequince`
  (bind _sequence_ (`self.Sequence `)
    (:`then`
      (bind (_outactor _returnvalue) (`LevelSequencePlayer.CreateLevelSequencePlayer` _sequence_))
      (`MovieSceneSequencePlayer.Play` _returnvalue)
      (`self.Active/Deactive Interaction` false)
      (if (> (`self.Time active next button`) 0.0)
        (`KismetSystemLibrary.Delay` (`self.Time active next button`))
        (`self.Active next sequence`)))
    (:`else`)))

(event `Event Press button`
  (params (`Down?` :type Boolean))
  (if `Down?`
    (bind (_direction _relative_location_sphere) (`Timeline|Press button` :!label _label)
      (:`Update`
        (`SceneComponent.K2_SetRelativeLocation` (`self.Sphere`) _relative_location_sphere false false))
      (:`Finished`
        (if `Down?`
          (`self.Event Press button` false)
          (`self.Active Sequince`))))
    (else
      (goto _label :!via `Reverse`))))

(event `/Game/Blueprint/Libraries/Interface/Char_Info.Interact`
  (params (Interact :type "/Game/Blueprint/Data/Enum/ETypeInteract Enum" :default "NewEnumerator0"))
  (switch `/Game/Blueprint/Data/Enum/ETypeInteract` Interact
    (:`NewEnumerator0`
      (if (not (`self.Active "press button"`))
        (`self.Event Press button` true)
        (set `self.Active "press button"` true)
        (set `self.Active?` false)))))

(fn `Active Button`
  (params (`Active?` :type Boolean)))

(fn `Active next sequence`
  (locals (Button :type "/Game/Blueprint/InteractionPlayer/Button Object Reference"))
  (bind _outactors (`GameplayStatics.GetAllActorsOfClass` "Button_C"))
  (for _array_element _outactors
    (bind _output_get (set `local.Button` _array_element))
    (if (== (`/Game/Blueprint/InteractionPlayer/Button.Sequence` _output_get) (+ (`self.Sequence`) 1))
      (`self.Active/Deactive Interaction` (`local.Button`) true)
      (break))))

(fn `Active/Deactive Interaction`
  (params (`Active?` :type Boolean))
  (`parent.Active/Deactive Interaction` `Active?`)
  (`self.Set info Widget`))

(fn `Get info seq`
  (bind _outrownames (`DataTableFunctionLibrary.GetDataTableRowNames` "/Game/Blueprint/Data/DataTable/SequenseDataTable.SequenseDataTable"))
  (bind _returnvalue (`|GetDataTableRow` "/Game/Blueprint/Data/DataTable/SequenseDataTable.SequenseDataTable" (`|GetArrayItem` _outrownames (`self.Sequence`)))
    (:`then`
      (set `self.Sequence ` (break `/Game/Blueprint/Data/Struct/Level_sequenceTime` _returnvalue))
      (set `self.Time active next button` (`.Timeactivenextbutton_5_5F0D796845DD8CFC5532CF8EFDB58BDE` (break `/Game/Blueprint/Data/Struct/Level_sequenceTime` _returnvalue))))))

(fn `Set index`
  (bind _outactors (`GameplayStatics.GetAllActorsOfClass` "Button_C"))
  (for _array_element _outactors
    (if (and (== (`self.Sequence`) (`/Game/Blueprint/InteractionPlayer/Button.Sequence` _array_element)) (!= _array_element self))
      (set `self.Sequence` -1))))

(fn `Set info Widget`
  (bind _astext_w (cast `/Game/Blueprint/Ui/TextW` (`WidgetComponent.GetWidget` (`self.Widget`))))
  (`/Game/Blueprint/Ui/TextW.Set Text` _astext_w (`KismetTextLibrary.Conv_StringToText` (`KismetStringLibrary.Concat_StrStr` "Кнопка " (`KismetStringLibrary.Conv_IntToString` (+ (`self.Sequence`) 1)))) (select `bool` (`self.Active?`) :`false` (struct :`R` 1.0 :`A` 1.0) :`true` (struct :`G` 1.0 :`A` 1.0) :!type "LinearColor Structure") 24))

(fn `UserConstructionScript`
  (`parent.UserConstructionScript`)
  (`self.Set index`)
  (`self.Get info seq`)
  (`self.Set info Widget`))