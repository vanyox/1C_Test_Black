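; AI point-of-interest actor holding local points, each paired with an animation montage and a wait value, plus a widget text label.
; Construction updates the label and nudges the montage and wait arrays toward the point count; BeginPlay refreshes the label.
; A debug event, whose only starting call is disconnected, spawns skeletal meshes at the points, yawed relative to the actor's center, and replays each montage on completion.
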(event `self.ReceiveBeginPlay`
  (`self.Set text`))

(event `Debug Anim`
  (params (`Loop?` :type Boolean) (Index :type Integer))
  (if `Loop?`
    (bind (_skmesh__ _anim_montage _index_out) (`self.Debug Get anim` `Loop?` (stale _array_element) (select `bool` `Loop?` :`false` (stale _array_index) :`true` Index) :!label _label))
    (`|PlayMontage` _skmesh__ _anim_montage
      (:`OnCompleted`
        (`self.Debug Anim` true _index_out)))
    (else
      (for (_array_element _array_index) (`self.Point (General)`)
        (goto _label)))))

(fn `Debug Get anim`
  (params (`Loop?` :type Boolean) (InputPin :type "Vector Structure") (`Index in` :type Integer))
  (returns (`SkMesh  ` :type "SkeletalMeshComponent Object Reference") (`Anim montage` :type "AnimMontage Object Reference") (`Index out` :type Integer))
  (locals (SkMesh :type "Array of SkeletalMeshComponent Object Reference"))
  (bind _returnvalue (`self.K2_GetActorLocation`))
  (bind _index_in (`local.Index in`))
  (bind _index_in_2 (`local.Index in`))
  (bind (_returnvalue_roll _returnvalue_pitch _returnvalue_yaw) (`KismetMathLibrary.BreakRotator` (`KismetMathLibrary.FindLookAtRotation` (+ InputPin _returnvalue) _returnvalue)))
  (if `Loop?`
    (return (`|GetArrayItem` (`self.DebugSkMesh`) _index_in) (`|GetArrayItem` (`self.PointAnim`) _index_in) (`local.Index in`))
    (else
      (`/Engine/EditorBlueprintResources/StandardMacros.IsValid` (`|GetArrayItem` (`self.DebugSkMesh`) (`local.Index in`))
        (:`Is Valid`
          _)
        (:`Is Not Valid`
          (bind _returnvalue_2 (`AddComponent|NODE_AddSkeletalMeshComponent-2` :`RelativeTransform` (`KismetMathLibrary.MakeTransform` InputPin (`KismetMathLibrary.MakeRotator` 0.0 0.0 (+ _returnvalue_yaw 270.0)))))
          (`KismetArrayLibrary.Array_Add` (`self.DebugSkMesh`) _returnvalue_2)))
      (return (`|GetArrayItem` (`self.DebugSkMesh`) _index_in_2) (`|GetArrayItem` (`self.PointAnim`) _index_in_2) (`local.Index in`)))))

(fn `Set Mass`
  (bind _wait_point (`self.wait point`))
  (bind _pointanim (`self.PointAnim`))
  (bind _returnvalue (`KismetArrayLibrary.Array_LastIndex` (`self.Point (General)`)))
  (for _ (`self.Point (General)`)
    (`|ExecutionSequence`
      (:`then_0`
        (if (< (`KismetArrayLibrary.Array_LastIndex` (`self.PointAnim`)) _returnvalue)
          (`KismetArrayLibrary.Array_Add` (`self.PointAnim`))
          (elif (!= (`KismetArrayLibrary.Array_LastIndex` (`self.PointAnim`)) (`KismetArrayLibrary.Array_LastIndex` (`self.Point (General)`)))
            (`KismetArrayLibrary.Array_Remove` _pointanim (`KismetArrayLibrary.Array_LastIndex` _pointanim)))))
      (:`then_1`
        (if (< (`KismetArrayLibrary.Array_LastIndex` (`self.wait point`)) _returnvalue)
          (`KismetArrayLibrary.Array_Add` (`self.wait point`))
          (elif (!= (`KismetArrayLibrary.Array_LastIndex` (`self.PointAnim`)) (`KismetArrayLibrary.Array_LastIndex` (`self.wait point`)))
            (`KismetArrayLibrary.Array_Remove` _wait_point (`KismetArrayLibrary.Array_LastIndex` _wait_point))))))))

(fn `Set text`
  (bind _astext_w (cast `/Game/Blueprint/Ui/TextW` (`WidgetComponent.GetWidget` (`self.Widget`))))
  (`/Game/Blueprint/Ui/TextW.Set Text` _astext_w (`self.In Text`) (`self.Specified Color`) (`self.In Font Info Size`)))

(fn `UserConstructionScript`
  (`self.Set text`)
  (`self.Set Mass`))